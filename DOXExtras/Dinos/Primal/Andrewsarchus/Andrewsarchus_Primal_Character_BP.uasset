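; Primal Andrewsarchus dino character Blueprint that adds death-buff handling and attack rules on top of its parent.
; On lethal damage it deactivates LH-type buffs, applies a death buff and returns whether that buff was added.
; Only attack indices 0 and 3 are allowed, against conscious characters for AI, or when tamed and un-netted for riders.
; Speed boost defers to the parent check but is blocked while the death buff is active.
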(fn ConstructionScript
  (|CallParentFunction))

(fn BPonLethalDamage
  (params (KillingDamage :type Float%20%28single-precision%29) (DamageEvent :type Damage%20Event%20Structure%20%28by%20ref%29) (Killer :type Controller%20Object%20Reference) (DamageCauser :type Actor%20Object%20Reference))
  (Class|PrimalCharacter|DeactivateBuffs (Variables|Default|GetLHBuffType) 0 false)
  (bind _returnvalue (Class|PrimalBuff|StaticAddBuff (Variables|Dino|GetDeathBuffClass) self 0 0 false))
  (return (Utilities|IsValid _returnvalue)))

(fn BlueprintCanAttack
  (params (AttackIndex :type Integer) (distance :type Float%20%28single-precision%29) (attackRangeOffset :type Float%20%28single-precision%29) (OtherTarget :type Actor%20Object%20Reference))
  (switch int AttackIndex
    (:Default
      _)
    (:0
      (bind _asprimalcharacter (Utilities|Casting|CastToPrimalCharacter OtherTarget :!label _label)
        (:then
          (if (Class|PrimalCharacter|BPIsConscious _asprimalcharacter)
            (LocalVariables|SetRetVal true)))
        (:CastFailed
          _)))
    (:1
      _)
    (:2
      _)
    (:3
      (goto _label))
    (:4
      _)
    (:5
      _))
  (return (LocalVariables|GetRetVal)))

(fn BlueprintCanRiderAttack
  (params (AttackIndex :type Integer))
  (if (and (Class|PrimalDinoCharacter|BPIsTamed) (not (CallFunction|HasNettedBuff)))
    (switch int AttackIndex
      (:Default
        _)
      (:0
        (LocalVariables|SetRetVal true :!label _label))
      (:1
        _)
      (:2
        _)
      (:3
        (goto _label))
      (:4
        _)
      (:5
        _)))
  (return (LocalVariables|GetRetVal)))

(fn CheckCanSpeedBoost
  (bind _canspeedboost (|CallParentFunction))
  (bind _isbuffactive (Dino|IsActiveDeathBuff))
  (return (and (not _isbuffactive) _canspeedboost)))

(fn IsActiveDeathBuff
  (bind _returnvalue (Class|PrimalCharacter|HasBuff (Variables|Dino|GetDeathBuffClass) true))
  (return _returnvalue))