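; Prime Andrewsarchus dino character that loots its kills, moving all victim items into its own inventory, and caps incoming damage and torpor.
; The damage override calls the parent but discards its result, capping the raw incoming value.
; Its HUD shows saddle minigun ammo, boost charges, slide-boost cooldown and water sinking when tamed.
; Untamed, it shows left/right steering prompts, taming progress, and effectiveness with a rider-clear timer bar.
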(event EventBPKilledSomethingEvent
  (params (killedTarget :type Primal%20Character%20Object%20Reference))
  (CallFunction|OnKillSomething killedTarget))

(fn ConstructionScript
  (|CallParentFunction))

(fn BPGetHUDElements
  (params (ForPC :type Player%20Controller%20Object%20Reference))
  (bind _returnvalue (Class|Actor|GetWorld))
  (bind _returnvalue_2 (Class|VictoryCore|GetNetworkTimeinSeconds))
  (bind _desiredturndirindex (Variables|Default|GetDesiredTurnDirIndex))
  (bind _tamingprogresshudelement (Variables|Default|GetTamingProgressHUDElement))
  (bind _tamingeffectivenesshudelement (Variables|Default|GetTamingEffectivenessHUDElement))
  (bind _currenttameaffinity (Variables|Default|GetCurrentTameAffinity))
  (bind _requiredtameaffinity (Variables|Default|GetRequiredTameAffinity))
  (bind _cleartamingridertime (Variables|Default|GetClearTamingRiderTime))
  (bind _tamingclearriderminmax (Variables|Default|GetTamingClearRiderMinMax))
  (bind _taminglefthudelement (Variables|Default|GetTamingLeftHUDElement))
  (bind _lasttamingmovedirection (Variables|Default|GetLastTamingMoveDirection))
  (bind _lasttamingmovedirection_2 (Variables|Default|GetLastTamingMoveDirection))
  (bind _miniammoitemclass (Variables|Default|GetMiniAmmoItemClass))
  (bind _tamingrighthudelement (Variables|Default|GetTamingRightHUDElement))
  (bind _myinventorycomponent (Variables|Default|GetMyInventoryComponent))
  (bind _lastexitslidemaxspeedboosttime (Variables|Default|GetLastExitSlideMaxSpeedBoostTime))
  (bind _exitslidemaxspeedboostregentime (Variables|Default|GetExitSlideMaxSpeedBoostRegenTime))
  (bind _numspeedboosts (Variables|Default|GetNumSpeedBoosts))
  (bind _maxspeedboosts (Variables|Default|GetMaxSpeedBoosts))
  (bind _speedboostregentime (Variables|Default|GetSpeedBoostRegenTime))
  (bind _desiredturndirindex_2 (Variables|Default|GetDesiredTurnDirIndex))
  (bind (_biseditoronly _brespectplayeruiscalesetting _btitleisextendedinfo _blabelisextendedinfo _title _textalignment_title _label _textalignment_label _textcontainerhorizontalalignment _textcontainerverticalalignment _zorder _progress _textcolor _textscale _textpadding _backgroundimagecolor _progresscolor _progressbarfilltype _anchormode _anchor _location _boverridelocationforuiscaling _locationatminscale _locationatdefaultscale _locationatmaxscale _size _scale _backgroundimage _progressbarfillimage _progressbarpadding _progressbarscale _icon _iconsize _iconscale _iconcolor _iconpadding _iconrotation _progressbarfillimagemargin _progressbarbackgroundimagemargin) (Utilities|Struct|BreakHUDElement _tamingrighthudelement))
  (bind (_biseditoronly_2 _brespectplayeruiscalesetting_2 _btitleisextendedinfo_2 _blabelisextendedinfo_2 _title_2 _textalignment_title_2 _label_2 _textalignment_label_2 _textcontainerhorizontalalignment_2 _textcontainerverticalalignment_2 _zorder_2 _progress_2 _textcolor_2 _textscale_2 _textpadding_2 _backgroundimagecolor_2 _progresscolor_2 _progressbarfilltype_2 _anchormode_2 _anchor_2 _location_2 _boverridelocationforuiscaling_2 _locationatminscale_2 _locationatdefaultscale_2 _locationatmaxscale_2 _size_2 _scale_2 _backgroundimage_2 _progressbarfillimage_2 _progressbarpadding_2 _progressbarscale_2 _icon_2 _iconsize_2 _iconscale_2 _iconcolor_2 _iconpadding_2 _iconrotation_2 _progressbarfillimagemargin_2 _progressbarbackgroundimagemargin_2) (Utilities|Struct|BreakHUDElement _tamingprogresshudelement))
  (bind (_biseditoronly_3 _brespectplayeruiscalesetting_3 _btitleisextendedinfo_3 _blabelisextendedinfo_3 _title_3 _textalignment_title_3 _label_3 _textalignment_label_3 _textcontainerhorizontalalignment_3 _textcontainerverticalalignment_3 _zorder_3 _progress_3 _textcolor_3 _textscale_3 _textpadding_3 _backgroundimagecolor_3 _progresscolor_3 _progressbarfilltype_3 _anchormode_3 _anchor_3 _location_3 _boverridelocationforuiscaling_3 _locationatminscale_3 _locationatdefaultscale_3 _locationatmaxscale_3 _size_3 _scale_3 _backgroundimage_3 _progressbarfillimage_3 _progressbarpadding_3 _progressbarscale_3 _icon_3 _iconsize_3 _iconscale_3 _iconcolor_3 _iconpadding_3 _iconrotation_3 _progressbarfillimagemargin_3 _progressbarbackgroundimagemargin_3) (Utilities|Struct|BreakHUDElement _tamingeffectivenesshudelement))
  (bind (_biseditoronly_4 _brespectplayeruiscalesetting_4 _btitleisextendedinfo_4 _blabelisextendedinfo_4 _title_4 _textalignment_title_4 _label_4 _textalignment_label_4 _textcontainerhorizontalalignment_4 _textcontainerverticalalignment_4 _zorder_4 _progress_4 _textcolor_4 _textscale_4 _textpadding_4 _backgroundimagecolor_4 _progresscolor_4 _progressbarfilltype_4 _anchormode_4 _anchor_4 _location_4 _boverridelocationforuiscaling_4 _locationatminscale_4 _locationatdefaultscale_4 _locationatmaxscale_4 _size_4 _scale_4 _backgroundimage_4 _progressbarfillimage_4 _progressbarpadding_4 _progressbarscale_4 _icon_4 _iconsize_4 _iconscale_4 _iconcolor_4 _iconpadding_4 _iconrotation_4 _progressbarfillimagemargin_4 _progressbarbackgroundimagemargin_4) (Utilities|Struct|BreakHUDElement _taminglefthudelement))
  (bind _returnvalue_3 (== _numspeedboosts _maxspeedboosts))
  (bind _returnvalue_4 (Class|VictoryCore|TimeSinceNetwork _returnvalue _lastexitslidemaxspeedboosttime))
  (bind _returnvalue_5 (== _lasttamingmovedirection _desiredturndirindex))
  (bind _returnvalue_6 (== _desiredturndirindex 1))
  (bind _returnvalue_7 (== _lasttamingmovedirection_2 _desiredturndirindex_2))
  (bind _returnvalue_8 (== _desiredturndirindex_2 2))
  (bind _returnvalue_9 (/ _currenttameaffinity _requiredtameaffinity))
  (bind _returnvalue_10 (- _cleartamingridertime _returnvalue_2))
  (bind _returnvalue_11 (Class|KismetMathLibrary|MapRange _returnvalue_4 0.0 _exitslidemaxspeedboostregentime 0.0 1.0))
  (bind _returnvalue_12 (Math|Conversions|ToFloat(Integer) _returnvalue_10))
  (bind _returnvalue_13 (and _returnvalue_5 _returnvalue_6))
  (bind _returnvalue_14 (and _returnvalue_7 _returnvalue_8))
  (bind _returnvalue_15 (Math|Float|Clamp(Float) _returnvalue_11))
  (bind _returnvalue_16 (Class|KismetMathLibrary|MapRange _returnvalue_12 (.x _tamingclearriderminmax) 0.0 0.0 1.0))
  (Utilities|FlowControl|Sequence
    (:then_0
      (if (Class|PrimalDinoCharacter|BPIsTamed)
        (bind _returnvalue_17 (Class|PrimalInventoryComponent|GetItemTemplateQuantity (Variables|Default|GetMyInventoryComponent) _miniammoitemclass 0 true false false false))
        (bind _returnvalue_18 (Class|PrimalInventoryComponent|GetItemTemplateQuantity (Variables|/Script/ShooterGame.PrimalCharacter|GetMyInventoryComponent (Variables|Default|GetRider)) _miniammoitemclass 0 true false false false))
        (bind _returnvalue_19 (Class|PrimalGameData|BPGetGameData))
        (bind _returnvalue_20 (Class|VictoryCore|GetClassDefaultObject (Variables|/Script/ShooterGame.PrimalGameData|GetGlobalUIDataClass _returnvalue_19)))
        (bind _asglobaluidata_bp_c (Utilities|Casting|CastToGlobalUIData_BP _returnvalue_20))
        (Utilities|IsValid _myinventorycomponent
          (:Is%20Valid
            (bind _returnvalue_21 (Class|PrimalInventoryComponent|GetEquippedItemOfType _myinventorycomponent "DinoSaddle"))
            (Utilities|IsValid _returnvalue_21
              (:Is%20Valid
                (bind _outhudelement (Default|BPGetHUDElementsModuleFuelorAmmo _asglobaluidata_bp_c 0 (Math|Integer|SelectInt (Math|Integer|SelectInt 0 1 (Variables|Default|GetbMinigunActive)) 2 (> (+ _returnvalue_17 _returnvalue_18) 0)) (Math|Float|SelectFloat 1.0 0.0 (> (+ _returnvalue_17 _returnvalue_18) 0)) (Utilities|String|ToString(Text) (Utilities|Text|FormatText (Variables|Default|GetAmmoFormatText) (Utilities|Text|ToText(String) (Utilities|String|ToString(Integer) (Math|Integer|Min(Integer) _returnvalue_18 999999))) (Utilities|Text|ToText(String) (Utilities|String|ToString(Integer) (Math|Integer|Min(Integer) _returnvalue_17 999999))))) (Utilities|String|SelectString "TURRET" "(YOU)" (> _returnvalue_17 0)) (Variables|Minigun|GetMiniAmmoItemIcon)))
                (Utilities|Array|Add (LocalVariables|GetRetElements) _outhudelement))
              (:Is%20Not%20Valid
                _)))
          (:Is%20Not%20Valid
            _))
        (bind _outhudelement_2 (Default|BPGetHUDElementsModuleFuelorAmmo _asglobaluidata_bp_c 1 (Math|Integer|SelectInt 0 (Math|Integer|SelectInt 2 1 (== _numspeedboosts 0)) _returnvalue_3) (Math|Float|SelectFloat 1.0 (Math|Float|Clamp(Float) (Class|KismetMathLibrary|MapRange (.Remainder (Math|Float|Division(WholeandRemainder) (Class|VictoryCore|TimeSinceNetwork (Class|Actor|GetWorld) (Variables|Default|GetLastSpeedBoostRegenTime)) _speedboostregentime)) 0.0 _speedboostregentime 0.0 1.0)) _returnvalue_3) (Utilities|String|ToString(Integer) _numspeedboosts) "CHARGES" "/Game/PrimalEarth/UI/Textures/StatsIcons/ArkG_AbilityIcons_AndrewsarchusHighBoost.ArkG_AbilityIcons_AndrewsarchusHighBoost"))
        (Utilities|Array|Add (LocalVariables|GetRetElements) _outhudelement_2)
        (bind _outhudelement_3 (Default|BPGetHUDElementsModuleFuelorAmmo _asglobaluidata_bp_c 2 (Math|Integer|SelectInt 0 2 (== _returnvalue_15 1.0)) _returnvalue_15 "" "SLIDE BOOST" "/Game/PrimalEarth/UI/Textures/StatsIcons/ArkG_AbilityIcons_AndrewsarchusLowBoost.ArkG_AbilityIcons_AndrewsarchusLowBoost"))
        (Utilities|Array|Add (LocalVariables|GetRetElements) _outhudelement_3)
        (if (Variables|Default|GetbShouldUnderwaterSink)
          (bind _outhudelement_4 (Default|BPGetHUDElementsModuleFuelorAmmo _asglobaluidata_bp_c 3 0 1.0 "" "WATER SINKING" "/Game/Fjordur/Icons/Buffs/ArkG_AbilityIcons_AndrewsarchusBottomWalk.ArkG_AbilityIcons_AndrewsarchusBottomWalk"))
          (Utilities|Array|Add (LocalVariables|GetRetElements) _outhudelement_4))
        (else
          (LocalVariables|SetLocalElement (Utilities|Struct|MakeHUDElement "ProgressBar" true _biseditoronly_4 _brespectplayeruiscalesetting_4 _btitleisextendedinfo_4 _blabelisextendedinfo_4 _title_4 _textalignment_title_4 _label_4 _textalignment_label_4 _textcontainerhorizontalalignment_4 _textcontainerverticalalignment_4 _zorder_4 (Math|Float|SelectFloat 1.0 0.0 _returnvalue_14) _textcolor_4 _textscale_4 _textpadding_4 (Math|Color|SelectColor "(R=0.000000,G=1.000000,B=0.000000,A=1.000000)" (Math|Color|SelectColor "(R=1.000000,G=0.000000,B=0.000000,A=1.000000)" (Math|Color|SelectColor "(R=1.000000,G=1.000000,B=1.000000,A=1.000000)" "(R=1.000000,G=1.000000,B=1.000000,A=0.100000)" (and (== _lasttamingmovedirection_2 2) (!= _desiredturndirindex_2 2))) (and _returnvalue_8 (!= _lasttamingmovedirection_2 _desiredturndirindex_2))) _returnvalue_14) _progresscolor_4 _progressbarfilltype_4 _anchormode_4 _anchor_4 _location_4 _boverridelocationforuiscaling_4 _locationatminscale_4 _locationatdefaultscale_4 _locationatmaxscale_4 _size_4 _scale_4 _backgroundimage_4 _progressbarfillimage_4 _progressbarpadding_4 _progressbarscale_4 _icon_4 _iconsize_4 _iconscale_4 _iconcolor_4 _iconpadding_4 _iconrotation_4 _progressbarfillimagemargin_4 _progressbarbackgroundimagemargin_4))
          (Utilities|Array|Add (LocalVariables|GetRetElements) (LocalVariables|GetLocalElement))
          (LocalVariables|SetLocalElement (Utilities|Struct|MakeHUDElement "ProgressBar" true _biseditoronly _brespectplayeruiscalesetting _btitleisextendedinfo _blabelisextendedinfo _title _textalignment_title _label _textalignment_label _textcontainerhorizontalalignment _textcontainerverticalalignment _zorder (Math|Float|SelectFloat 1.0 0.0 _returnvalue_13) _textcolor _textscale _textpadding (Math|Color|SelectColor "(R=0.000000,G=1.000000,B=0.000000,A=1.000000)" (Math|Color|SelectColor "(R=1.000000,G=0.000000,B=0.000000,A=1.000000)" (Math|Color|SelectColor "(R=1.000000,G=1.000000,B=1.000000,A=1.000000)" "(R=1.000000,G=1.000000,B=1.000000,A=0.100000)" (and (== _lasttamingmovedirection 1) (!= _desiredturndirindex 1))) (and _returnvalue_6 (!= _lasttamingmovedirection _desiredturndirindex))) _returnvalue_13) _progresscolor _progressbarfilltype _anchormode _anchor _location _boverridelocationforuiscaling _locationatminscale _locationatdefaultscale _locationatmaxscale _size _scale _backgroundimage _progressbarfillimage _progressbarpadding _progressbarscale _icon _iconsize _iconscale _iconcolor _iconpadding _iconrotation _progressbarfillimagemargin _progressbarbackgroundimagemargin))
          (Utilities|Array|Add (LocalVariables|GetRetElements) (LocalVariables|GetLocalElement))
          (LocalVariables|SetLocalElement (Utilities|Struct|MakeHUDElement "ProgressBar" true _biseditoronly_2 _brespectplayeruiscalesetting_2 _btitleisextendedinfo_2 _blabelisextendedinfo_2 (Utilities|String|ToString(Text) (Utilities|Text|FormatText "Taming: {1}%" (Utilities|Text|ToText(Float) (* _returnvalue_9 1e+02) "HalfToEven" true 1 324 1 1))) _textalignment_title_2 _label_2 _textalignment_label_2 _textcontainerhorizontalalignment_2 _textcontainerverticalalignment_2 _zorder_2 _returnvalue_9 _textcolor_2 _textscale_2 _textpadding_2 _backgroundimagecolor_2 _progresscolor_2 _progressbarfilltype_2 _anchormode_2 _anchor_2 _location_2 _boverridelocationforuiscaling_2 _locationatminscale_2 _locationatdefaultscale_2 _locationatmaxscale_2 _size_2 _scale_2 _backgroundimage_2 _progressbarfillimage_2 _progressbarpadding_2 _progressbarscale_2 _icon_2 _iconsize_2 _iconscale_2 _iconcolor_2 _iconpadding_2 _iconrotation_2 _progressbarfillimagemargin_2 _progressbarbackgroundimagemargin_2))
          (Utilities|Array|Add (LocalVariables|GetRetElements) (LocalVariables|GetLocalElement))
          (LocalVariables|SetLocalElement (Utilities|Struct|MakeHUDElement "ProgressBar" true _biseditoronly_3 _brespectplayeruiscalesetting_3 _btitleisextendedinfo_3 _blabelisextendedinfo_3 (Utilities|String|ToString(Text) (Utilities|Text|FormatText "Taming Effectiveness: {1}%" (Utilities|Text|ToText(Float) (* (/ 1.0 (+ (* (Variables|Default|GetTameIneffectivenessModifier) (Variables|/Script/ShooterGame.PrimalCharacterStatusComponent|GetTamingIneffectivenessMultiplier (Variables|Default|GetMyCharacterStatusComponent))) 1.0)) 1e+02) "HalfToEven" true 1 324 1 1))) _textalignment_title_3 _label_3 _textalignment_label_3 _textcontainerhorizontalalignment_3 _textcontainerverticalalignment_3 _zorder_3 _returnvalue_16 _textcolor_3 _textscale_3 _textpadding_3 _backgroundimagecolor_3 (Math|Color|Lerp(LinearColor) "(R=1.000000,G=0.020000,B=0.020000,A=0.750000)" "(R=1.000000,G=0.020000,B=0.020000,A=0.750000)" _returnvalue_16) _progressbarfilltype_3 _anchormode_3 _anchor_3 _location_3 _boverridelocationforuiscaling_3 _locationatminscale_3 _locationatdefaultscale_3 _locationatmaxscale_3 _size_3 _scale_3 _backgroundimage_3 _progressbarfillimage_3 _progressbarpadding_3 _progressbarscale_3 _icon_3 _iconsize_3 _iconscale_3 _iconcolor_3 _iconpadding_3 _iconrotation_3 _progressbarfillimagemargin_3 _progressbarbackgroundimagemargin_3))
          (Utilities|Array|Add (LocalVariables|GetRetElements) (LocalVariables|GetLocalElement)))))
    (:then_1
      (return (LocalVariables|GetRetElements)))))

(fn OnKillSomething
  (params (KilledTarget :type Primal%20Character%20Object%20Reference))
  (Class|PrimalInventoryComponent|TransferAllItemstoInventory (Variables|/Script/ShooterGame.PrimalCharacter|GetMyInventoryComponent KilledTarget) (Variables|Default|GetMyInventoryComponent))
  (return))

(fn BPAdjustDamage
  (params (IncomingDamage :type Float%20%28single-precision%29) (TheDamageEvent :type Damage%20Event%20Structure) (EventInstigator :type Controller%20Object%20Reference) (DamageCauser :type Actor%20Object%20Reference) (bIsPointDamage :type Boolean) (PointHitInfo :type Hit%20Result%20Structure))
  (bind _damagereceivedcap (Variables|Damage|GetDamageReceivedCap))
  (|CallParentFunction IncomingDamage TheDamageEvent EventInstigator DamageCauser bIsPointDamage PointHitInfo)
  (return (Math|Float|SelectFloat _damagereceivedcap IncomingDamage (< _damagereceivedcap IncomingDamage))))

(fn BPAdjustTorpidityDamage
  (params (DesiredTorpidityDamage :type Float%20%28single-precision%29) (HealthDamageAmount :type Float%20%28single-precision%29) (DamageType :type Damage%20Type%20Class%20Reference))
  (bind _torporreceivedcap (Variables|Damage|GetTorporReceivedCap))
  (return (Math|Float|SelectFloat _torporreceivedcap DesiredTorpidityDamage (< _torporreceivedcap DesiredTorpidityDamage))))