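; Ancient Andrewsarchus character variant whose server-side minigun fire adds a projectile at each shot's impact point, via ServerFireAOEMinigun.
; Shots pass safe-location and can-fire checks, with interval throttling only on dedicated servers; failed checks cancel firing.
; A line trace applies point damage scaled by weapon stat, then spawns the projectile at the hit or max range and multicasts VFX.
; Ammo comes from the dino's inventory, falling back to the rider's.
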(event Custom|Server_FireMinigun
  (params (Location :type Vector) (Direction :type Vector))
  (CallFunction|ServerFireAOEMinigun Location Direction))

(fn ConstructionScript
  (|CallParentFunction))

(fn ServerFireAOEMinigun
  (params (Location :type Vector) (Direction :type Vector))
  (bind _returnvalue (Math|Vector|Normalize Direction))
  (bind _self self)
  (bind _myinventorycomponent (Variables|Default|GetMyInventoryComponent))
  (bind _miniammoitemclass (Variables|Default|GetMiniAmmoItemClass))
  (bind _rider (Variables|Default|GetRider))
  (bind _maxminigundistance (Variables|Default|GetMaxMinigunDistance))
  (bind _minigunfireinterval (Variables|Default|GetMinigunFireInterval))
  (bind _returnvalue_2 (* _returnvalue _maxminigundistance))
  (bind _returnvalue_3 (+ Location _returnvalue_2))
  (if (Networking|IsDedicatedServer)
    (if (Class|VictoryCore|IsTimeSinceNetwork (Class|Actor|GetWorld) (Variables|Default|GetLastMinigunFireTime) (- _minigunfireinterval (* _minigunfireinterval 0.1)) true)
      (Variables|Default|SetLastMinigunFireTime (Class|VictoryCore|GetNetworkTimeinSeconds))
      (if (CallFunction|IsServerSafeFiringLocation Location) :!label _label
        (bind _canenable (CallFunction|GetCanEnableMinigun))
        (if _canenable
          (bind _canshoot (CallFunction|GetCanShootMinigun))
          (if _canshoot
            (Utilities|FlowControl|Sequence
              (:then_0
                (Class|PrimalCharacter|ForceUpdateAimedCharacters (Class|Actor|GetWorld) Location _returnvalue_3 0 false 2e+03)
                (bind (_outhit _returnvalue_4) (Collision|LineTraceByChannel Location _returnvalue_3 "ECC_GameTraceChannel1" true (Utilities|Array|MakeArray _rider) "None"))
                (if _returnvalue_4
                  (bind _returnvalue_5 (Class|PrimalInventoryComponent|GetTotalEquippedItemStat (Variables|Default|GetMyInventoryComponent) "WeaponDamagePercent"))
                  (Game|Damage|ApplyPointDamage (.HitActor (Collision|BreakHitResult _outhit)) (* (Variables|Default|GetBaseMinigunDamage) _returnvalue_5) _returnvalue _outhit (Pawn|GetController) self (Variables|Default|GetMinigunDamageType) 0.0 false "ECC_GameTraceChannel1"))
                (bind _returnvalue_6 (Class|VictoryCore|SpawnActorDeferred (Variables|Minigun|GetMinigunProjectileType) (Class|Actor|GetWorld) (Math|Vector|SelectVector (.Location (Collision|BreakHitResult _outhit)) _returnvalue_3 _returnvalue_4) (Math|Conversions|RotationFromXVector _returnvalue) _self _self true))
                (bind _asshooterprojectile (Utilities|Casting|CastToShooterProjectile _returnvalue_6)
                  (:then
                    (Class|ShooterProjectile|BPInitVelocity _asshooterprojectile _returnvalue))
                  (:CastFailed
                    _))
                (Class|VictoryCore|FinishSpawning _returnvalue_6)
                (CallFunction|MultiSpawnFireVFX (Math|Vector|SelectVector (.Location (Collision|BreakHitResult _outhit)) _returnvalue_3 _returnvalue_4) Location _returnvalue _outhit))
              (:then_1
                (if (not (Variables|Default|GetbMinigunFiring))
                  (Variables|Default|SetbMinigunFiring true true)))
              (:then_2
                (bind _returnvalue_7 (Class|PrimalInventoryComponent|GetItemTemplateQuantity _myinventorycomponent _miniammoitemclass 0 true false false false))
                (if (> _returnvalue_7 0)
                  (Class|PrimalInventoryComponent|BPIncrementItemTemplateQuantity _myinventorycomponent _miniammoitemclass -1 true false true false false false 0 false)
                  (else
                    (Class|PrimalInventoryComponent|BPIncrementItemTemplateQuantity (Variables|/Script/ShooterGame.PrimalCharacter|GetMyInventoryComponent _rider) _miniammoitemclass -1 true false true false false false 0 false)))))
            (else
              (CallFunction|ServerCancelMinigunFire :!label _label_2)))
          (else
            (goto _label_2)))
        (else
          (goto _label_2))))
    (else
      (goto _label))))